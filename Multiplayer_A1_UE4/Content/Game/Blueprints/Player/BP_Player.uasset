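; Player pawn for a networked Bomberman game that moves by input axes and drops bombs via a server event on Space.
; Damage passes through a server event to a multicast, which decrements Health and grants temporary immunity.
; A MultiGate seeded by Health swaps the mesh's emissive dynamic material from its initial green to yellow, red or black.
; At zero Health, a server event travels to the game-over map.
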(event Custom|Server_SpawnBomb
  (params (Spawn%20Position :type Vector))
  (bind _self self)
  (Game|SpawnActorfromClass "/Game/Game/Blueprints/Bomb/BP_Bomb.BP_Bomb_C" (Math|Transform|MakeTransform Spawn%20Position "0, 0, 0" "1,1,1") "Undefined" _self _self))

(event Custom|Server_TakeDamage
  (Networking|SwitchHasAuthority
    (:Authority
      (CallFunction|MulticastTakeDamage))))

(event Custom|Multicast_TakeDamage
  (if (Variables|Default|GetCan%20Receive%20Damage)
    (Utilities|FlowControl|Sequence
      (:then_0
        (bind _result (Math|Integer|DecrementInt (Variables|Default|GetHealth))
          (:%20%20
            (bind _output_get (Variables|Default|SetHealth (Math|Integer|Clamp(Integer) _result 0 3)))
            (Utilities|FlowControl|Sequence
              (:then_0
                (if (== (Variables|Default|GetHealth) 0)
                  (CallFunction|ServerTravel)))
              (:then_1
                (Variables|Default|SetCan%20Receive%20Damage false)
                (Development|PrintString (Utilities|String|ToString(Integer) _output_get))
                (Utilities|FlowControl|Delay (Variables|Default|GetImmortal%20Timer))
                (Variables|Default|SetCan%20Receive%20Damage true))))))
      (:then_1
        (Utilities|FlowControl|MultiGate false false (Variables|Default|GetHealth)
          (:Out%200
            (bind _returnvalue (Rendering|Material|CreateDynamicMaterialInstance (Variables|Character|GetMesh) 0 "/Game/Game/Blueprints/Materials/MI_Black.MI_Black" "None" :!class /Script/Engine.PrimitiveComponent))
            (bind _output_get_2 (Variables|Default|SetMID_Cube _returnvalue))
            (Rendering|Material|SetScalarParameterValue _output_get_2 "Emission" 0.0 :!class /Script/Engine.MaterialInstanceDynamic))
          (:Out%201
            (bind _returnvalue_2 (Rendering|Material|CreateDynamicMaterialInstance (Variables|Character|GetMesh) 0 "/Game/Game/Blueprints/Materials/MI_Red.MI_Red" "None" :!class /Script/Engine.PrimitiveComponent))
            (bind _output_get_3 (Variables|Default|SetMID_Cube _returnvalue_2))
            (Rendering|Material|SetScalarParameterValue _output_get_3 "Emission" 5.0 :!class /Script/Engine.MaterialInstanceDynamic))
          (:Out%202
            (bind _returnvalue_3 (Rendering|Material|CreateDynamicMaterialInstance (Variables|Character|GetMesh) 0 "/Game/Game/Blueprints/Materials/MI_Yellow.MI_Yellow" "None" :!class /Script/Engine.PrimitiveComponent))
            (bind _output_get_4 (Variables|Default|SetMID_Cube _returnvalue_3))
            (Rendering|Material|SetScalarParameterValue _output_get_4 "Emission" 2.5 :!class /Script/Engine.MaterialInstanceDynamic)))))))

(event Custom|Server_Travel
  (bind _asgi_bomberman (Utilities|Casting|CastToGI_Bomberman (Game|GetGameInstance)))
  (Default|ServerTravelMap _asgi_bomberman "Map_GameOver")
  (Development|PrintString "ir pro game over mapa"))

(event EventBeginPlay
  (bind _returnvalue (Rendering|Material|CreateDynamicMaterialInstance (Variables|Character|GetMesh) 0 "/Game/Game/Blueprints/Materials/MI_Green.MI_Green" "None" :!class /Script/Engine.PrimitiveComponent))
  (bind _output_get (Variables|Default|SetMID_Cube _returnvalue))
  (Rendering|Material|SetScalarParameterValue _output_get "Emission" (Variables|Default|GetEmission%20Base%20Value) :!class /Script/Engine.MaterialInstanceDynamic)
  (if (Pawn|IsLocallyControlled)
    (Viewport|RemoveAllWidgets)))

(event EventTick
  (params (DeltaSeconds :type Float%20%28single-precision%29))
  (Pawn|Input|AddMovementInput (Math|Vector|MakeVector (Input|AxisValues|GetMoveForward) (Input|AxisValues|GetMoveRight) 0.0) 1.0 false))

(event EventTakeDamage
  (CallFunction|ServerTakeDamage))

(event Input|KeyboardEvents|SpaceBar
  (params (Key :type Key%20Structure :default "None"))
  (:Pressed
    (CallFunction|ServerSpawnBomb (Transformation|GetActorLocation))))

(fn ConstructionScript)

(fn OnRepHealth)