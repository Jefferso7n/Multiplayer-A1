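; BP_Bomb is a networked timed bomb that explodes in a cross pattern.
; On BeginPlay the authority waits TimeUntilExplosion, then triggers the explosion through a multicast.
; The explosion event spawns BP_Explosion actors at fixed offsets from the bomb mesh, two steps along each horizontal axis direction with none at the center, then destroys the bomb.
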(event Custom|Multicast_Explode
  (for _array_element (Utilities|Array|MakeArray "100.000000, 0, 0" "0,100.000000, 0" "-100.000000,0.000000,0.000000" "0.000000,-100.000000, 0" "200.000000,0.000000,0.000000" "0.000000,200.000000,0.000000" "-200.000000,0.000000,0.000000" "0.000000,-200.000000, 0")
    (Game|SpawnActorfromClass "/Game/Game/Blueprints/Bomb/BP_Explosion.BP_Explosion_C" (Math|Transform|MakeTransform (+ (Transformation|GetWorldLocation (Variables|Default|GetBombMesh)) _array_element) "0, 0, 0" "1,1,1") "Undefined" 0 0))
  (Actor|DestroyActor))

(event EventBeginPlay
  (Networking|SwitchHasAuthority
    (:Authority
      (Utilities|FlowControl|Delay (Variables|Default|GetTime%20Until%20Explosion))
      (CallFunction|MulticastExplode))))

(fn ConstructionScript)