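; BP_Explosion is a bomb explosion actor that damages pawns and destructibles within a radius.
; All logic runs once on BeginPlay, using a sphere overlap at the actor's location and sending TakeDamageMessage, with no damage amount, to each actor found.
; It also draws a temporary debug sphere at that radius and spawns the P_Explosion particle effect.
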(event EventBeginPlay
  (Utilities|FlowControl|Sequence
    (:then_0
      (Rendering|Debug|DrawDebugSphere (Transformation|GetActorLocation) (Variables|Default|GetSphere%20Radius) 8 "(R=1.000000,G=0.250000,B=0.000000,A=1.000000)" 3.0 8.0))
    (:then_1
      (bind (_outactors _returnvalue) (Collision|SphereOverlapActors (Transformation|GetActorLocation) (Variables|Default|GetSphere%20Radius) (Utilities|Array|MakeArray "ObjectTypeQuery3" "ObjectTypeQuery6") 0))
      (if _returnvalue
        (for _array_element _outactors
          (Class|BPIDamageable|TakeDamage(Message) _array_element))))
    (:then_2
      (Effects|SpawnEmitteratLocation "/Game/StarterContent/Particles/P_Explosion.P_Explosion" (Transformation|GetActorLocation)))))

(fn ConstructionScript)